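; Player-controlled cleaner Blueprint that displays one of three tool kits (cleaning, vacuum or welding) and handles the HUD and pausing.
; BeginPlay adds the HUD widget, and the Pause input pauses the game, opens the pause menu and shows the mouse cursor.
; Tick polls KitNumber to set kit visibility and uses Interacting as the rotating cleaning kit's play rate, so it animates only during interaction.
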(event EventBeginPlay
  (bind _returnvalue (UserInterface|CreateWidget "/Game/UI/WidgetHUD.WidgetHUD_C"))
  (UserInterface|Viewport|AddtoViewport _returnvalue 0))

(event EventTick
  (params (DeltaSeconds :type Float%20%28single-precision%29))
  (bind _cleaningkit_rotating (Variables|Default|GetCleaningKit_Rotating))
  (bind _kitnumber (Variables|Default|GetKitNumber))
  ;[1 1 1] Sets the meshes for kits to visible, and checks if the cleaning kit should rotate.
  (Rendering|SetVisibility _cleaningkit_rotating (== _kitnumber 1) false)
  (Rendering|SetVisibility (Variables|Default|GetVacuumKit) (== _kitnumber 2) false)
  (Rendering|SetVisibility (Variables|Default|GetKit_Welding) (== _kitnumber 3) false)
  (Components|Timeline|SetPlayRate _cleaningkit_rotating (Math|Conversions|ToFloat(Boolean) (Variables|Default|GetInteracting))))

(event Input|ActionEvents|InputActionPause
  (params (Key :type Key%20Structure :default "AnyKey"))
  (bind _returnvalue (Game|GetPlayerController 0))
  (:Pressed
    (Game|SetGamePaused true)
    (bind _returnvalue_2 (UserInterface|CreateWidget "/Game/UI/PauseMenu.PauseMenu_C" _returnvalue))
    (UserInterface|Viewport|AddtoViewport _returnvalue_2 0)
    (Variables|/Script/Engine.PlayerController|SetbShowMouseCursor _returnvalue true)))

(fn ConstructionScript)